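; Terrain tile for an endless level that fills itself with props and enemy pawns on BeginPlay through PlaceActors and PlaceAIPawns.
; Its barrier starts locked red, turns green and passable while the player overlaps the locking volume, and relocks on exit.
; First entry reports the tile conquered to InfinitrGameMode.
; The player reaching the destroy volume makes the game mode spawn another tile and destroys this one; an arrow provides the attach transform.
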(event OnComponentBeginOverlap(lockingvolume)
  (params (OverlappedComponent :type Primitive%20Component%20Object%20Reference) (OtherActor :type Actor%20Object%20Reference) (OtherComp :type Primitive%20Component%20Object%20Reference) (OtherBodyIndex :type Integer) (bFromSweep :type Boolean) (SweepResult :type Hit%20Result%20Structure%20%28by%20ref%29))
  (Utilities|Actor OtherActor)
  (Utilities|FlowControl|Sequence
    (:then_0
      (CallFunction|Unlock))
    (:then_1
      (CallFunction|Tileconquered))))

(event OnComponentEndOverlap(lockingvolume)
  (params (OverlappedComponent :type Primitive%20Component%20Object%20Reference) (OtherActor :type Actor%20Object%20Reference) (OtherComp :type Primitive%20Component%20Object%20Reference) (OtherBodyIndex :type Integer))
  (Utilities|Actor OtherActor)
  (CallFunction|Lock))

(event OnComponentBeginOverlap(destroyvolume)
  (params (OverlappedComponent :type Primitive%20Component%20Object%20Reference) (OtherActor :type Actor%20Object%20Reference) (OtherComp :type Primitive%20Component%20Object%20Reference) (OtherBodyIndex :type Integer) (bFromSweep :type Boolean) (SweepResult :type Hit%20Result%20Structure%20%28by%20ref%29))
  (Utilities|Actor OtherActor)
  (bind _asinfinitr_game_mode (Utilities|Casting|CastToInfinitrGameMode (Game|GetGameMode)))
  (Default|SpawnTile _asinfinitr_game_mode)
  (Actor|DestroyActor))

(event EventBeginPlay
  (CallFunction|Lock)
  (Class|Tile|PlaceActors "/Game/dynamic/Terrain/props/Container_BP.Container_BP_C" 1 5 4e+02 1.0 1.0)
  (Class|Tile|PlaceActors "/Game/dynamic/Terrain/props/Rock_05_BP.Rock_05_BP_C" 1 3 2.5e+02 1.0 1.0)
  (Class|Tile|PlaceActors "/Game/dynamic/Terrain/props/Canister1_BP.Canister1_BP_C" 1 6 2.5e+02 1.0 2.0)
  (Class|Tile|PlaceActors "/Game/dynamic/Terrain/props/Rock_17_BP.Rock_17_BP_C" 1 2 2.5e+02 1.0 1.0)
  (Class|Tile|PlaceActors "/Game/dynamic/Terrain/props/Sack1_BP.Sack1_BP_C" 1 3 2.5e+02 1.0 1.0)
  (Class|Tile|PlaceActors "/Game/dynamic/Terrain/props/supply_BP.supply_BP_C" 1 4 2.5e+02 1.0 3.0)
  (Class|Tile|PlaceAIPawns "/Game/dynamic/character/Behaviour/character.character_C" (Variables|Default|Getminenemies) (Variables|Default|Getmaxenemies) 2.5e+02))

(event Collision|EventActorBeginOverlap
  (params (OtherActor :type Actor%20Object%20Reference)))

(event EventTick
  (params (DeltaSeconds :type Float%20%28single-precision%29)))

(fn ConstructionScript)

(fn Attachlocation
  (return (Transformation|GetWorldTransform (Variables|Default|GetArrow))))

(fn Unlock
  (Collision|SetCollisionEnabled (Variables|Default|Getbarrier) "NoCollision")
  (Rendering|Material|SetMaterial (Variables|Default|Getbarrier) 0 "/Game/dynamic/Terrain/greenbarrier.greenbarrier"))

(fn Lock
  (Collision|SetCollisionEnabled (Variables|Default|Getbarrier) "QueryAndPhysics")
  (Rendering|Material|SetMaterial (Variables|Default|Getbarrier) 0 "/Game/dynamic/Terrain/redbarrier.redbarrier"))

(fn Tileconquered
  (if (not (Variables|Default|Getistileconqured))
    (bind _asinfinitr_game_mode (Utilities|Casting|CastToInfinitrGameMode (Game|GetGameMode)))
    (Default|Newtileconquerd _asinfinitr_game_mode)
    (Variables|Default|Setistileconqured true)))